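; Trigger volume that plays a Level Sequencer cutscene once, swapping the player's sprite and HUD for cinematic UI.
; Overlap starts the sequence and locks movement; Tick detects playback or completion to apply or restore that state, and PastCine skips to the end.
; During playback, ChangeColor ping-pongs a dynamic material's BricksColor alpha.
; CollectMasterPieces instead blends to CamActor, stops the piece's movement, plays the sequence, then triggers SceneLoader.
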(event `PastCine`
  (bind _mat (`self.Mat`))
  (bind _lvsequencer (`self.LVSequencer`))
  (bind _maincharacter (`self.MainCharacter`))
  ;[1 1 1] Level Sequencer Part
  (`/Engine/EditorBlueprintResources/StandardMacros.IsValid` _lvsequencer
    (:`Is Valid`
      (`MovieSceneSequencePlayer.GoToEndAndStop` (`LevelSequenceActor.SequencePlayer` _lvsequencer))
      (set `self.isAlreadyPlay` true)
      (set `self.Play` false)
      (`Controller.ResetIgnoreMoveInput` (`GameplayStatics.GetPlayerController` 0))
      (`SceneComponent.SetVisibility` (`/Game/SpaceSchoolAdventure/BP/Character/Player/MainCharacter_BP.PaperSprite` (`self.MainCharacter`)) true false)
      (`Widget.RemoveFromParent` (`/Game/SpaceSchoolAdventure/BP/Character/Player/MainCharacter_BP.UI_Cine` _maincharacter))
      (`UserWidget.AddToViewport` (`/Game/SpaceSchoolAdventure/BP/Character/Player/MainCharacter_BP.UI_MainUser` _maincharacter) 0)
      (set `/Game/SpaceSchoolAdventure/BP/Character/Player/MainCharacter_BP.TriggerCam` null _maincharacter)
      (`/Engine/EditorBlueprintResources/StandardMacros.IsValid` _mat
        (:`Is Valid`
          (`MaterialInstanceDynamic.SetVectorParameterValue` _mat "BricksColor" (make `LinearColor` 0.0)))))))

(event `self.CollisionComponent.OnComponentBeginOverlap`
  (params (OverlappedComponent :type "PrimitiveComponent Object Reference") (OtherActor :type "Actor Object Reference") (OtherComp :type "PrimitiveComponent Object Reference") (OtherBodyIndex :type Integer) (bFromSweep :type Boolean) (SweepResult :type "HitResult Structure (by ref)"))
  (bind _maincharacter (`self.MainCharacter`))
  (bind _lvsequencer (`self.LVSequencer`))
  (bind _ui_cine (`/Game/SpaceSchoolAdventure/BP/Character/Player/MainCharacter_BP.UI_Cine` (`self.MainCharacter`)))
  ;[1 1 1] Level Sequencer Part
  (if (not (`self.isAlreadyPlay`))
    (set `self.Play` true)
    (bind _asmain_character_bp (cast `/Game/SpaceSchoolAdventure/BP/Character/Player/MainCharacter_BP` OtherActor))
    (bind _output_get (set `self.MainCharacter` _asmain_character_bp))
    (set `/Game/SpaceSchoolAdventure/BP/Character/Player/MainCharacter_BP.TriggerCam` self _output_get)
    (`Widget.RemoveFromParent` (`/Game/SpaceSchoolAdventure/BP/Character/Player/MainCharacter_BP.UI_Dialogs` _maincharacter))
    (`Widget.RemoveFromParent` (`/Game/SpaceSchoolAdventure/BP/Character/Player/MainCharacter_BP.UI_MainUser` _maincharacter))
    (`Controller.SetIgnoreMoveInput` (`GameplayStatics.GetPlayerController` 0) true)
    (`SceneComponent.SetVisibility` (`/Game/SpaceSchoolAdventure/BP/Character/Player/MainCharacter_BP.PaperSprite` (`self.MainCharacter`)) false false)
    (set `self.TriggerCine` true)
    (`UserWidget.AddToViewport` _ui_cine 0)
    (`/Game/SpaceSchoolAdventure/BP/UI/UI_Cameracine.Flashing` _ui_cine)
    (`/Engine/EditorBlueprintResources/StandardMacros.IsValid` _lvsequencer
      (:`Is Valid`
        (`MovieSceneSequencePlayer.Play` (`LevelSequenceActor.SequencePlayer` _lvsequencer))))))

(event `self.ReceiveTick`
  (params (DeltaSeconds :type "Float (single-precision)"))
  (bind _mat (`self.Mat`))
  (bind _maincharacter (`self.MainCharacter`))
  (bind _lvsequencer (`self.LVSequencer`))
  (bind _maincharacter_2 (`self.MainCharacter`))
  (bind _ui_cine (`/Game/SpaceSchoolAdventure/BP/Character/Player/MainCharacter_BP.UI_Cine` (`self.MainCharacter`)))
  ;[1 1 1] Level Sequencer Part
  (if (not (`self.isAlreadyPlay`))
    (`/Engine/EditorBlueprintResources/StandardMacros.IsValid` _lvsequencer
      (:`Is Valid`
        (if (`MovieSceneSequencePlayer.IsPlaying` (`LevelSequenceActor.SequencePlayer` _lvsequencer))
          (`self.ChangeColor` DeltaSeconds)
          (if (not (`self.Play`))
            (set `self.Play` true)
            (bind _asmain_character_bp (cast `/Game/SpaceSchoolAdventure/BP/Character/Player/MainCharacter_BP` (`GameplayStatics.GetPlayerCharacter` 0)))
            (bind _output_get (set `self.MainCharacter` _asmain_character_bp))
            (set `/Game/SpaceSchoolAdventure/BP/Character/Player/MainCharacter_BP.TriggerCam` self _output_get)
            (`Widget.RemoveFromParent` (`/Game/SpaceSchoolAdventure/BP/Character/Player/MainCharacter_BP.UI_Dialogs` _maincharacter_2))
            (`Widget.RemoveFromParent` (`/Game/SpaceSchoolAdventure/BP/Character/Player/MainCharacter_BP.UI_MainUser` _maincharacter_2))
            (`SceneComponent.SetVisibility` (`/Game/SpaceSchoolAdventure/BP/Character/Player/MainCharacter_BP.PaperSprite` (`self.MainCharacter`)) false false)
            (`UserWidget.AddToViewport` _ui_cine 0)
            (`/Game/SpaceSchoolAdventure/BP/UI/UI_Cameracine.Flashing` _ui_cine))
          (else
            (`/Engine/EditorBlueprintResources/StandardMacros.IsValid` (`self.MainCharacter`)
              (:`Is Valid`
                (set `self.isAlreadyPlay` true)
                (set `self.Play` false)
                (`Controller.ResetIgnoreMoveInput` (`GameplayStatics.GetPlayerController` 0))
                (`SceneComponent.SetVisibility` (`/Game/SpaceSchoolAdventure/BP/Character/Player/MainCharacter_BP.PaperSprite` (`self.MainCharacter`)) true false)
                (`Widget.RemoveFromParent` (`/Game/SpaceSchoolAdventure/BP/Character/Player/MainCharacter_BP.UI_Cine` _maincharacter))
                (`UserWidget.AddToViewport` (`/Game/SpaceSchoolAdventure/BP/Character/Player/MainCharacter_BP.UI_MainUser` _maincharacter) 0)
                (set `/Game/SpaceSchoolAdventure/BP/Character/Player/MainCharacter_BP.TriggerCam` null _maincharacter)
                (`/Engine/EditorBlueprintResources/StandardMacros.IsValid` _mat
                  (:`Is Valid`
                    (`MaterialInstanceDynamic.SetVectorParameterValue` _mat "BricksColor" (make `LinearColor` 0.0))))))))))))

(event `ChangeColor`
  (params (DeltaTime :type "Float (double-precision)"))
  (`/Engine/EditorBlueprintResources/StandardMacros.IsValid` (`self.Actor`)
    (:`Is Valid`
      (`|ExecutionSequence`
        (:`then_0`
          (`/Engine/EditorBlueprintResources/StandardMacros.DoOnce` false
            (:`Completed`
              (bind _returnvalue (`KismetMaterialLibrary.CreateDynamicMaterialInstance` "/Game/SpaceSchoolAdventure/Texture/WallFloor_Inst_2.WallFloor_Inst_2"))
              (set `self.Mat` _returnvalue)
              (`PrimitiveComponent.SetMaterial` (`/Game/SpaceSchoolAdventure/BP/Interactables/ButtonDoor.Cube` (`self.Actor`)) 0 _returnvalue))))
        (:`then_1`
          (bind _returnvalue_2 (`MaterialInstanceDynamic.K2_GetVectorParameterValue` (`self.Mat`) "BricksColor"))
          (`MaterialInstanceDynamic.SetVectorParameterValue` (`self.Mat`) "BricksColor" (make `LinearColor` 0.0 0.0 0.0 (+ (`.A` (break `LinearColor` _returnvalue_2)) (* (`self.Speed`) DeltaTime))))
          ;[1 1 1] PingPong Effect
          (if (> (`.A` (break `LinearColor` _returnvalue_2)) 1.0)
            (`/Engine/EditorBlueprintResources/StandardMacros.DoOnce` false :!label _label
              (:`Completed`
                (`|ExecutionSequence`
                  (:`then_0`
                    (goto _label_3 :!via `Reset`))
                  (:`then_1`
                    (`/Engine/EditorBlueprintResources/StandardMacros.NegateFloat` (`self.Speed`) :!label _label_2)))))
            (elif (< (`.A` (break `LinearColor` _returnvalue_2)) 0.0)
              (`/Engine/EditorBlueprintResources/StandardMacros.DoOnce` false :!label _label_3
                (:`Completed`
                  (`|ExecutionSequence`
                    (:`then_0`
                      (goto _label_2))
                    (:`then_1`
                      (goto _label :!via `Reset`))))))))))))

(event `CollectMasterPieces`
  (params (Character :type "Actor Object Reference"))
  (bind _sceneloader (`self.SceneLoader`))
  (bind _timetotranslate (`self.TimeToTranslate`))
  (bind _sequenceplayer (`LevelSequenceActor.SequencePlayer` (`self.LVSequencer`)))
  (bind _returnvalue (`MovieSceneSequencePlayer.GetDuration` _sequenceplayer))
  ;[1 1 1] CamRig Part
  (if (not (`self.isAlreadyPlay`))
    (set `self.Play` true)
    (bind _asmain_character_bp (cast `/Game/SpaceSchoolAdventure/BP/Character/Player/MainCharacter_BP` Character))
    (bind _output_get (set `self.MainCharacter` _asmain_character_bp))
    (set `/Game/SpaceSchoolAdventure/BP/Character/Player/MainCharacter_BP.TriggerCam` self _output_get)
    (`Widget.RemoveFromParent` (`/Game/SpaceSchoolAdventure/BP/Character/Player/MainCharacter_BP.UI_MainUser` (`self.MainCharacter`)))
    (`SceneComponent.SetVisibility` (`/Game/SpaceSchoolAdventure/BP/Character/Player/MainCharacter_BP.PaperSprite` (`self.MainCharacter`)) false false)
    (`PlayerController.SetViewTargetWithBlend` (`GameplayStatics.GetPlayerController` 0) (`self.CamActor`) _timetotranslate "VTBlend_Linear" 0.0 false)
    (`KismetSystemLibrary.Delay` _timetotranslate)
    (`InterpToMovementComponent.StopSimulating` (`/Game/SpaceSchoolAdventure/BP/Collectable/MasterPiece_BP.InterpToMovement` (`self.MasterPiece`)) (`GameplayStatics.MakeHitResult` false))
    (`MovieSceneSequencePlayer.Play` _sequenceplayer)
    (`KismetSystemLibrary.Delay` (`KismetMathLibrary.Conv_IntToDouble` (/ (break `FrameNumber` (break `QualifiedFrameTime` _returnvalue)) (`KismetMathLibrary.BreakFrameRate` (`.FrameRate` (break `QualifiedFrameTime` _returnvalue))))))
    (`MovieSceneSequencePlayer.Pause` _sequenceplayer)
    (`/Engine/EditorBlueprintResources/StandardMacros.IsValid` _sceneloader
      (:`Is Valid`
        (`/Game/SpaceSchoolAdventure/BP/SceneLoading/SceneLoader.LoadLevel` _sceneloader Character)))))

(fn `UserConstructionScript`)