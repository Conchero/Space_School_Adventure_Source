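; Louis is a character that hovers in place and performs an electric attack on enemies.
; Two timelines move its mesh along hover and attack splines, each playing forward, then reversing.
; An attack impulse only sets a flag, so the strike waits until the hover cycle returns to its start.
; Louis then turns toward the target, triggers the enemy's electric field and sound at the spline's end, retreats, and resumes hovering.
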(event `self.ReceiveBeginPlay`
  (`self.PlaySplineForward`))

(event `PlaySplineForward`
  (bind _splinehoover (`self.SplineHoover`))
  (set `self.isSplinePlayingFwd` true)
  (bind (_direction _zvalue) (`Timeline|TimelineHoover` :!label _label)
    (:`Update`
      (`SceneComponent.K2_SetWorldLocation` (`self.mesh`) (`SplineComponent.GetLocationAtDistanceAlongSpline` _splinehoover (* _zvalue (`SplineComponent.GetSplineLength` _splinehoover)) "World") false false))
    (:`Finished`
      (if (`self.isSplinePlayingFwd`)
        (`self.PlaySplineBack`)
        (elif (`self.isAttackPlayingFwd`)
          (`self.PlayAttackForward`)
          (else
            (`self.PlaySplineForward`)))))))

(event `PlaySplineBack`
  (set `self.isSplinePlayingFwd` false)
  (goto _label :!via `Reverse`))

(event `self.BP_ATKImpulseEvent`
  (params (_enemy :type "Ennemie Object Reference") (_lookAtRotation :type "Rotator Structure"))
  (set `self.isAttackPlayingFwd` true))

(event `PlayAttackForward`
  (bind _splineattack (`self.SplineAttack`))
  (`self.K2_SetActorRotation` (stale `self.BP_ATKImpulseEvent` _lookAtRotation))
  (bind (_direction _zvalue) (`Timeline|TimelineAttack` :!label _label_2)
    (:`Update`
      (`SceneComponent.K2_SetWorldLocation` (`self.mesh`) (`SplineComponent.GetLocationAtDistanceAlongSpline` _splineattack (* _zvalue (`SplineComponent.GetSplineLength` _splineattack)) "World") false false))
    (:`Finished`
      (if (`self.isAttackPlayingFwd`)
        (`/Engine/EditorBlueprintResources/StandardMacros.IsValid` (stale `self.BP_ATKImpulseEvent` _enemy)
          (:`Is Valid`
            (`Ennemie.ShowElectricField` (stale `self.BP_ATKImpulseEvent` _enemy))
            (`self.PlayElectricSound`)
            (`self.PlayAttackBack`))
          (:`Is Not Valid`
            (`self.PlayAttackBack`)))
        (else
          (`self.K2_SetActorRelativeRotation` (struct))
          (`self.PlaySplineForward`))))))

(event `PlayAttackBack`
  (set `self.isAttackPlayingFwd` false)
  (goto _label_2 :!via `Reverse`))

(event `PlayElectricSound`
  (bind _audiocomponent (`self.audioComponent`))
  (`AudioComponent.SetSound` _audiocomponent "/Game/SpaceSchoolAdventure/Sounds/Character/LouisAttack.LouisAttack")
  (`AudioComponent.Play` _audiocomponent 0.0))

(fn `UserConstructionScript`)