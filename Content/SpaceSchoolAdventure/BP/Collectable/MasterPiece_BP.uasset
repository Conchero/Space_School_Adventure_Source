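; Collectable master piece Blueprint for Space School Adventure.
; On collection by the player character, it disables that character's input and hands the character to TriggerCamera's CollectMasterPieces.
; A separate timer event sets CanCollect to true after a short delay.
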(event `self.Collect_BP`
  (params (actor :type "Actor Object Reference"))
  (bind _returnvalue (`GameplayStatics.GetPlayerCharacter` 0))
  (if (== actor _returnvalue)
    (bind _asmain_character (cast `MainCharacter` _returnvalue))
    (`self.DisableInput` _asmain_character (`GameplayStatics.GetPlayerController` 0))
    (`/Game/SpaceSchoolAdventure/BP/Camera/TriggerVolumeCamera_BP.CollectMasterPieces` (`self.TriggerCamera`) _asmain_character)))

(event `self.TimerBeforeCollect_BP`
  (`KismetSystemLibrary.Delay` 0.2)
  (set `self.canCollect` true))

(fn `UserConstructionScript`)