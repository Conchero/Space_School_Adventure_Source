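; Carriable cube Blueprint whose emissive glow pulses; the graph holds only this visual effect, with no carrying logic.
; Tick calls ChangeColor, which creates a dynamic material instance on the mesh once, then shifts its "emissive" parameter by Speed times delta time.
; A pair of DoOnce gates that reset each other is meant to ping-pong the glow, changing Speed at the upper and lower limits.
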(event `self.ReceiveBeginPlay`)

(event `self.ReceiveTick`
  (params (DeltaSeconds :type "Float (single-precision)"))
  (`self.ChangeColor` DeltaSeconds))

(event `ChangeColor`
  (params (DeltaTime :type "Float (double-precision)"))
  (`|ExecutionSequence`
    (:`then_0`
      (`/Engine/EditorBlueprintResources/StandardMacros.DoOnce` false
        (:`Completed`
          (bind _returnvalue (`KismetMaterialLibrary.CreateDynamicMaterialInstance` "/Game/Materials/box_portable_Inst.box_portable_Inst"))
          (set `self.Mat` _returnvalue)
          (`PrimitiveComponent.SetMaterial` (`self.mesh`) 0 _returnvalue))))
    (:`then_1`
      (bind _returnvalue_2 (`MaterialInstanceDynamic.K2_GetScalarParameterValue` (`self.Mat`) "emissive"))
      (`MaterialInstanceDynamic.SetScalarParameterValue` (`self.Mat`) "emissive" (+ _returnvalue_2 (* (`self.Speed`) DeltaTime)))
      ;[1 1 1] PingPong Effect
      (if (> _returnvalue_2 500.0)
        (`/Engine/EditorBlueprintResources/StandardMacros.DoOnce` false :!label _label
          (:`Completed`
            (`|ExecutionSequence`
              (:`then_0`
                (goto _label_3 :!via `Reset`))
              (:`then_1`
                (`/Engine/EditorBlueprintResources/StandardMacros.NegateFloat` (`self.Speed`) :!label _label_2)))))
        (elif (< _returnvalue_2 7.0)
          (`/Engine/EditorBlueprintResources/StandardMacros.DoOnce` false :!label _label_3
            (:`Completed`
              (`|ExecutionSequence`
                (:`then_0`
                  (goto _label_2))
                (:`then_1`
                  (goto _label :!via `Reset`))))))))))

(fn `UserConstructionScript`)