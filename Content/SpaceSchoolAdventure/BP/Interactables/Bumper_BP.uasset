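; Interactable bumper that springs the main character into the air, either as a free launch or along a guided path.
; When IsGuided, overlap starts a timeline that moves the character along the spline, facing its end, with OnBumper set until finished.
; Otherwise, a hit launches the character upward by Force, clears crushing and resets air control if crushing, with a brief lockout against repeat launches.
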(event `self.Sphere1.OnComponentBeginOverlap`
  (params (OverlappedComponent :type "PrimitiveComponent Object Reference") (OtherActor :type "Actor Object Reference") (OtherComp :type "PrimitiveComponent Object Reference") (OtherBodyIndex :type Integer) (bFromSweep :type Boolean) (SweepResult :type "HitResult Structure (by ref)"))
  (bind _spline (`self.Spline`))
  (bind _spline_2 (`self.Spline`))
  (bind (_returnvalue_roll _returnvalue_pitch) (`KismetMathLibrary.BreakRotator` (`self.K2_GetActorRotation` (`self.As Main Character BP`))))
  (bind (_returnvalue_roll_2 _returnvalue_pitch_2 _returnvalue_yaw) (`KismetMathLibrary.BreakRotator` (`KismetMathLibrary.FindLookAtRotation` (`SplineComponent.GetLocationAtSplinePoint` _spline 0 "World") (`SplineComponent.GetLocationAtSplinePoint` _spline (`SplineComponent.GetNumberOfSplinePoints` _spline_2) "World"))))
  (if (`self.isGuided`)
    (bind _asmain_character_bp (cast `/Game/SpaceSchoolAdventure/BP/Character/Player/MainCharacter_BP` OtherActor))
    (`GameplayStatics.PlaySound2D` "/Game/SpaceSchoolAdventure/Sounds/Character/BumperSpring.BumperSpring" 1.0 1.0 0.0 null null)
    (set `self.As Main Character BP` _asmain_character_bp)
    (set `MainCharacter.OnBumper` true (`self.As Main Character BP`))
    (bind (_direction _distancealongspline) (`Timeline|Track` :!via `PlayFromStart`)
      (:`Update`
        (`self.K2_SetActorLocationAndRotation` (`self.As Main Character BP`) (`SplineComponent.GetLocationAtDistanceAlongSpline` _spline_2 (* _distancealongspline (`SplineComponent.GetSplineLength` _spline_2)) "World") (`KismetMathLibrary.MakeRotator` _returnvalue_roll _returnvalue_pitch _returnvalue_yaw) false false))
      (:`Finished`
        (set `MainCharacter.OnBumper` false (`self.As Main Character BP`))))))

(event `self.Sphere.OnComponentHit`
  (params (HitComponent :type "PrimitiveComponent Object Reference") (OtherActor :type "Actor Object Reference") (OtherComp :type "PrimitiveComponent Object Reference") (NormalImpulse :type "Vector Structure") (Hit :type "HitResult Structure (by ref)"))
  (if (not (`self.isGuided`))
    (bind _asmain_character_bp (cast `/Game/SpaceSchoolAdventure/BP/Character/Player/MainCharacter_BP` OtherActor))
    (if (`MainCharacter.isCrushing` _asmain_character_bp)
      (set `self.ForceMultiplier` 1.0)
      (set `MainCharacter.isCrushing` false _asmain_character_bp)
      (set `CharacterMovementComponent.AirControl` 1.0 (`Character.CharacterMovement` _asmain_character_bp))
      (else
        (set `self.ForceMultiplier` 1.0)))
    (bind _output_get (set `self.As Main Character BP` _asmain_character_bp))
    (if (not (`self.IsLaunched`))
      (`Character.LaunchCharacter` _output_get (* (0.0 0.0 1.0) (* (`self.Force`) (`self.ForceMultiplier`))) false false)
      (set `self.IsLaunched` true)
      (`GameplayStatics.PlaySound2D` "/Game/SpaceSchoolAdventure/Sounds/Character/BumperSpring.BumperSpring" 1.0 1.0 0.0 null null)
      (`KismetSystemLibrary.Delay` 0.2)
      (set `self.IsLaunched` false))))

(fn `UserConstructionScript`)