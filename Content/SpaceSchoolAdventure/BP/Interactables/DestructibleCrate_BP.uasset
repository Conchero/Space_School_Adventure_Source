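; Destructible crate interactable that shatters with a sound, fades out and removes itself from the level.
; BeginPlay puts a dynamic instance of the Box material on the destructible mesh for fading.
; DestructionBP fractures the mesh with an impulse along the actor's right vector, ignores a custom collision channel and plays the destroyed sound.
; Once destroyed, Tick lowers Opacity by delta time until below zero, then destroys the actor.
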(event `self.ReceiveBeginPlay`
  (bind _returnvalue (`KismetMaterialLibrary.CreateDynamicMaterialInstance` "/Game/SpaceSchoolAdventure/Materials/box.box" "None"))
  (bind _output_get (set `self.Material` _returnvalue))
  (`PrimitiveComponent.SetMaterial` (`self.destructibleMesh`) 0 _output_get))

(event `self.ReceiveTick`
  (params (DeltaSeconds :type "Float (single-precision)"))
  (bind _material (`self.Material`))
  (if (`self.isDestroyed`)
    (bind _returnvalue (`MaterialInstanceDynamic.K2_GetScalarParameterValue` _material "Opacity"))
    (if (>= _returnvalue 0.0)
      (`MaterialInstanceDynamic.SetScalarParameterValue` _material "Opacity" (- _returnvalue DeltaSeconds))
      (else
        (`self.K2_DestroyActor`)))))

(event `self.Destruction_BP`
  (params (_character :type "MainCharacter Object Reference"))
  (bind _audiocomponent (`self.audioComponent`))
  (bind _destructiblemesh (`self.destructibleMesh`))
  (`DestructibleComponent.ApplyDamage` _destructiblemesh 100.0 (`self.K2_GetActorLocation`) (`self.GetActorRightVector`) 3000.0)
  (set `self.isDestroyed` true)
  (`PrimitiveComponent.SetCollisionResponseToChannel` _destructiblemesh "ECC_GameTraceChannel2" "ECR_Ignore")
  (`AudioComponent.SetSound` _audiocomponent "/Game/SpaceSchoolAdventure/Sounds/Character/DestructibleCrateDestroyed.DestructibleCrateDestroyed")
  (`AudioComponent.Play` _audiocomponent 0.0))

(fn `UserConstructionScript`)