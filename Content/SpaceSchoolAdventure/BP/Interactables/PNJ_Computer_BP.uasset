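; Computer NPC interactable that tailors its dialog to the player's level progress.
; On overlap it runs the parent logic, then, if the main character reference is valid, copies its SceneLoaderEnd value onto the character.
; It sets IndexOfList to the count of the character's unlocked levels and calls ChangeDialogs to update the dialog.
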(event `self.ReceiveBeginPlay`
  (`parent.ReceiveBeginPlay`))

(event `self.ReceiveActorBeginOverlap`
  (params (OtherActor :type "Actor Object Reference"))
  (bind _as_main_character_bp (`self.As Main Character BP`))
  (`parent.ReceiveActorBeginOverlap` OtherActor)
  (`/Engine/EditorBlueprintResources/StandardMacros.IsValid` _as_main_character_bp
    (:`Is Valid`
      (set `/Game/SpaceSchoolAdventure/BP/Character/Player/MainCharacter_BP.SceneLoaderEnd` (`self.SceneLoaderEnd`) _as_main_character_bp)
      (set `self.indexOfList` (`KismetArrayLibrary.Array_Length` (`MainCharacter.levelUnlocked` _as_main_character_bp)))
      (`self.Change Dialogs`))))

(fn `UserConstructionScript`
  (`parent.UserConstructionScript`))