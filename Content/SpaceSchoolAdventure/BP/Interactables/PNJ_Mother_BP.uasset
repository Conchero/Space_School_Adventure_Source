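; Interactable mother NPC that offers dialogue to the player in Space School Adventure.
; Overlapping the main character marks it as the interaction target and shows its dialog UI, while leaving clears the target and removes both dialog widgets.
; Its current dialogs come from a list entry chosen by index, set at BeginPlay and refreshed by a Change Dialogs function.
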(event `self.ReceiveActorBeginOverlap`
  (params (OtherActor :type "Actor Object Reference"))
  (bind _asmain_character_bp (cast `/Game/SpaceSchoolAdventure/BP/Character/Player/MainCharacter_BP` OtherActor))
  (bind _output_get (set `self.As Main Character BP` _asmain_character_bp))
  (set `MainCharacter.canInteract` true _output_get)
  (set `/Game/SpaceSchoolAdventure/BP/Character/Player/MainCharacter_BP.isInteractWith` self (`self.As Main Character BP`))
  (`UserWidget.AddToViewport` (`/Game/SpaceSchoolAdventure/BP/Character/Player/MainCharacter_BP.UI_Dialogs` _output_get) 0))

(event `self.ReceiveActorEndOverlap`
  (params (OtherActor :type "Actor Object Reference"))
  (bind _asmain_character_bp (cast `/Game/SpaceSchoolAdventure/BP/Character/Player/MainCharacter_BP` OtherActor))
  (bind _output_get (set `self.As Main Character BP` _asmain_character_bp))
  (set `MainCharacter.canInteract` false _output_get)
  (`Widget.RemoveFromParent` (`/Game/SpaceSchoolAdventure/BP/Character/Player/MainCharacter_BP.UI_Dialogs` _output_get))
  (`Widget.RemoveFromParent` (`/Game/SpaceSchoolAdventure/BP/Character/Player/MainCharacter_BP.Dialog` _output_get))
  (set `/Game/SpaceSchoolAdventure/BP/Character/Player/MainCharacter_BP.isInteractWith` null (`self.As Main Character BP`)))

(event `self.ReceiveBeginPlay`
  (set `self.Dialogs` (`.Dialogs_3_44F2614F423EA008798766A13D24049A` (break `/Game/SpaceSchoolAdventure/BP/Interactables/DialogsStruct` (`|GetArrayItem` (`self.ListOfDialog`) (`self.indexOfList`))))))

(fn `Change Dialogs`
  (set `self.Dialogs` (`.Dialogs_3_44F2614F423EA008798766A13D24049A` (break `/Game/SpaceSchoolAdventure/BP/Interactables/DialogsStruct` (`|GetArrayItem` (`self.ListOfDialog`) (`self.indexOfList`))))))

(fn `UserConstructionScript`)