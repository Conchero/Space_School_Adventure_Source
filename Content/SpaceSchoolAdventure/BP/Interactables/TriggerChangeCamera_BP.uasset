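; Trigger volume that switches the main character's camera to a fixed, raised view while the player is inside.
; On overlap it clears ActiveCamera, zeroes control rotation, disables spring arm collision, then saves and overrides the arm offset and camera rotation.
; On exit it restores those settings and sets control rotation to RotationCamera.
; BeginPlay also collects overlapping Pieces actors into PieceInstance, which this graph never reads.
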(event `self.ReceiveBeginPlay`
  (for _array_element (`PrimitiveComponent.GetOverlappingActors` (`self.CollisionComponent`) null)
    (bind _aspieces (cast `/Game/SpaceSchoolAdventure/BP/Collectable/Pieces` _array_element))
    (`KismetArrayLibrary.Array_AddUnique` (`self.PieceInstance`) _aspieces)))

(event `self.CollisionComponent.OnComponentBeginOverlap`
  (params (OverlappedComponent :type "PrimitiveComponent Object Reference") (OtherActor :type "Actor Object Reference") (OtherComp :type "PrimitiveComponent Object Reference") (OtherBodyIndex :type Integer) (bFromSweep :type Boolean) (SweepResult :type "HitResult Structure (by ref)"))
  (bind _asmain_character_bp (cast `/Game/SpaceSchoolAdventure/BP/Character/Player/MainCharacter_BP` OtherActor))
  (set `MainCharacter.activeCamera` false _asmain_character_bp)
  (`Controller.SetControlRotation` (`GameplayStatics.GetPlayerController` 0) (`KismetMathLibrary.MakeRotator` 0.0))
  (bind _springarm (`/Game/SpaceSchoolAdventure/BP/Character/Player/MainCharacter_BP.SpringArm` _asmain_character_bp))
  (set `SpringArmComponent.bDoCollisionTest` false _springarm)
  (set `MainCharacter.springArmValue` (`SpringArmComponent.SocketOffset` _springarm) _asmain_character_bp)
  (bind _camera (`/Game/SpaceSchoolAdventure/BP/Character/Player/MainCharacter_BP.Camera` _asmain_character_bp))
  (set `MainCharacter.cameraValue` (`SceneComponent.RelativeRotation` _camera) _asmain_character_bp)
  (set `SpringArmComponent.SocketOffset` (160.0 0.0 756.0) _springarm)
  (`SceneComponent.K2_SetRelativeRotation` _camera (struct :`Pitch` 290.0) false false))

(event `self.CollisionComponent.OnComponentEndOverlap`
  (params (OverlappedComponent :type "PrimitiveComponent Object Reference") (OtherActor :type "Actor Object Reference") (OtherComp :type "PrimitiveComponent Object Reference") (OtherBodyIndex :type Integer))
  (bind _asmain_character_bp (cast `/Game/SpaceSchoolAdventure/BP/Character/Player/MainCharacter_BP` OtherActor))
  (`Controller.SetControlRotation` (`GameplayStatics.GetPlayerController` 0) (`self.RotationCamera`))
  (set `MainCharacter.activeCamera` true _asmain_character_bp)
  (bind _springarm (`/Game/SpaceSchoolAdventure/BP/Character/Player/MainCharacter_BP.SpringArm` _asmain_character_bp))
  (set `SpringArmComponent.bDoCollisionTest` true _springarm)
  (set `SpringArmComponent.SocketOffset` (`MainCharacter.springArmValue` _asmain_character_bp) _springarm)
  (`SceneComponent.K2_SetRelativeRotation` (`/Game/SpaceSchoolAdventure/BP/Character/Player/MainCharacter_BP.Camera` _asmain_character_bp) (`MainCharacter.cameraValue` _asmain_character_bp) false false))

(fn `UserConstructionScript`)