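; One-shot trigger volume that shows a command prompt (text and image) on the player's Command widget.
; On the first MainCharacter_BP overlap it registers itself as the character's CommandTrigger, adds the widget and fills it with its Command text and Sprite.
; Tick counts up to TimerMax and removes the widget, but only while this volume is still the current CommandTrigger, so a newer trigger takes over dismissal.
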(event `self.CollisionComponent.OnComponentBeginOverlap`
  (params (OverlappedComponent :type "PrimitiveComponent Object Reference") (OtherActor :type "Actor Object Reference") (OtherComp :type "PrimitiveComponent Object Reference") (OtherBodyIndex :type Integer) (bFromSweep :type Boolean) (SweepResult :type "HitResult Structure (by ref)"))
  (bind _asmain_character_bp (cast `/Game/SpaceSchoolAdventure/BP/Character/Player/MainCharacter_BP` OtherActor))
  (if (not (`self.isAlreadyPlay`))
    (set `MainCharacter.commandTrigger` self _asmain_character_bp)
    (set `self.isEnter` true)
    (bind _command (`/Game/SpaceSchoolAdventure/BP/Character/Player/MainCharacter_BP.Command` _asmain_character_bp))
    (set `self.CommandLocal` _command)
    (`/Game/SpaceSchoolAdventure/BP/UI/TutoCommand.Add` _command)
    (`TextBlock.SetText` (`/Game/SpaceSchoolAdventure/BP/UI/TutoCommand.TextBlock_Command` _command) (`self.command`))
    (`Image.SetBrushFromTexture` (`/Game/SpaceSchoolAdventure/BP/UI/TutoCommand.Image_Command` _command) (`self.sprite`) false)
    (set `self.isAlreadyPlay` true)))

(event `self.ReceiveTick`
  (params (DeltaSeconds :type "Float (single-precision)"))
  (bind _asmain_character_bp (cast `/Game/SpaceSchoolAdventure/BP/Character/Player/MainCharacter_BP` (`GameplayStatics.GetPlayerCharacter` 0)))
  (if (and (`self.isEnter`) (== (`MainCharacter.commandTrigger` _asmain_character_bp) self))
    (bind _output_get (set `self.CurrentTimer` (+ DeltaSeconds (`self.CurrentTimer`))))
    (if (>= _output_get (`self.TimerMax`))
      (set `self.isEnter` false)
      (`/Game/SpaceSchoolAdventure/BP/UI/TutoCommand.Remove` (`self.CommandLocal`))
      (set `self.CurrentTimer` 0.0))))

(fn `UserConstructionScript`)