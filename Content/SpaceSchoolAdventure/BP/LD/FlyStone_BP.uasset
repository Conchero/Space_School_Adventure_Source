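; FlyStone is a floating stone actor that drifts vertically back and forth while slowly rotating.
; On BeginPlay it stores its start position, randomly picks an end point Distance above or below, and randomizes the spin direction of its RotatingMovement component.
; Tick drives a DoOnce and FlipFlop that alternately play and reverse the Translate timeline, which lerps the location and resets the gate when finished.
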(event `self.ReceiveBeginPlay`
  (bind (_returnvalue_x _returnvalue_y _returnvalue_z) (`KismetMathLibrary.BreakVector` (`self.K2_GetActorLocation`)))
  (bind _rotatingmovement (`self.RotatingMovement`))
  (bind _distance (`self.Distance`))
  (set `self.startPosition` (`self.K2_GetActorLocation`))
  (if (`KismetMathLibrary.RandomBool`)
    (set `self.endPosition` (`KismetMathLibrary.MakeVector` _returnvalue_x _returnvalue_y (+ _returnvalue_z _distance)))
    (else
      (set `self.endPosition` (`KismetMathLibrary.MakeVector` _returnvalue_x _returnvalue_y (- _returnvalue_z _distance)))))
  (if (`KismetMathLibrary.RandomBool`)
    (set `RotatingMovementComponent.RotationRate` (struct :`Yaw` -10.0) _rotatingmovement)
    (else
      (set `RotatingMovementComponent.RotationRate` (struct :`Yaw` 10.0) _rotatingmovement))))

(event `self.ReceiveTick`
  (params (DeltaSeconds :type "Float (single-precision)"))
  (`/Engine/EditorBlueprintResources/StandardMacros.DoOnce` false :!label _label
    (:`Completed`
      (`/Engine/EditorBlueprintResources/StandardMacros.FlipFlop`
        (:`A`
          (bind (_direction _position) (`Timeline|Translate` :!via `PlayFromStart` :!label _label_2)
            (:`Update`
              (`self.K2_SetActorLocation` (`KismetMathLibrary.VLerp` (`self.startPosition`) (`self.endPosition`) _position)))
            (:`Finished`
              (goto _label :!via `Reset`))))
        (:`B`
          (goto _label_2 :!via `Reverse`))))))

(fn `UserConstructionScript`)