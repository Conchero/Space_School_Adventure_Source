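; KillZone_BP is a kill volume that costs the main character one life and teleports them to their respawn checkpoint.
; On overlap it plays FadeIn and FadeOut level sequences sped up around the teleport, then destroys the sequence actors.
; An Ennemie damage branch hangs off the failed player cast, inside the exact player-class check, so enemies never reach it.
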(event `self.ReceiveActorBeginOverlap`
  (params (OtherActor :type "Actor Object Reference"))
  (if (== (`GameplayStatics.GetObjectClass` OtherActor) "/Game/SpaceSchoolAdventure/BP/Character/Player/MainCharacter_BP.MainCharacter_BP_C")
    (bind _outactor (`LevelSequencePlayer.CreateLevelSequencePlayer` "/Game/LoadingScreen/FadeIn.FadeIn"))
    (bind _sequenceplayer (`LevelSequenceActor.SequencePlayer` _outactor))
    (`MovieSceneSequencePlayer.SetPlayRate` _sequenceplayer 5.0)
    (`MovieSceneSequencePlayer.Play` _sequenceplayer)
    (`KismetSystemLibrary.Delay` 0.4)
    (`MovieSceneSequencePlayer.SetPlayRate` _sequenceplayer 1.0)
    (bind _asmain_character_bp (cast `/Game/SpaceSchoolAdventure/BP/Character/Player/MainCharacter_BP` OtherActor)
      (:`then`
        (bind _returnvalue (`MainCharacter.GetRespawnCheckpointPos` _asmain_character_bp))
        (`MainCharacter.RemoveLife` _asmain_character_bp 1 false "None")
        (`self.K2_SetActorLocation` OtherActor _returnvalue false true)
        (bind _outactor_2 (`LevelSequencePlayer.CreateLevelSequencePlayer` "/Game/LoadingScreen/FadeOut.FadeOut"))
        (bind _sequenceplayer_2 (`LevelSequenceActor.SequencePlayer` _outactor_2))
        (`MovieSceneSequencePlayer.SetPlayRate` _sequenceplayer_2 5.0)
        (`MovieSceneSequencePlayer.Play` _sequenceplayer_2)
        (`KismetSystemLibrary.Delay` 0.4)
        (`MovieSceneSequencePlayer.SetPlayRate` _sequenceplayer_2 1.0)
        (`/Engine/EditorBlueprintResources/StandardMacros.IsValid` _outactor
          (:`Is Valid`
            _)))
      (:`CastFailed`
        (bind _asennemie (cast `Ennemie` OtherActor))
        (`Ennemie.RemoveLife` _asennemie 100 null)))
    (`self.K2_DestroyActor` _outactor)
    (`/Engine/EditorBlueprintResources/StandardMacros.IsValid` _outactor_2
      (:`Is Valid`
        (`self.K2_DestroyActor` _outactor_2)))))

(fn `UserConstructionScript`)