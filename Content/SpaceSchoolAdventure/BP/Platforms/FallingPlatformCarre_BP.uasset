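; Square falling platform that provides the audio and material setup for its shake and fall phases.
; On BeginPlay it creates a dynamic instance of the platform material and stores it in Material.
; Sound events share one AudioComponent, swapping between shake and fall sounds, with the fall sound starting at an offset.
; Stopping the fall sound clears the component, while the stop-shaking event is empty; no movement logic lives in this graph.
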(event `self.ReceiveBeginPlay`
  (bind _returnvalue (`PrimitiveComponent.CreateDynamicMaterialInstance` (`self.Platform`) 0 "/Game/SpaceSchoolAdventure/Materials/platform/plateformcarre_Inst.plateformcarre_Inst" "None"))
  (set `self.Material` _returnvalue))

(event `self.PlayShakingSound_BP`
  (bind _audiocomponent (`self.audioComponent`))
  (`AudioComponent.SetSound` _audiocomponent "/Game/SpaceSchoolAdventure/Sounds/Character/FallingPlatformShake.FallingPlatformShake")
  (`AudioComponent.Play` _audiocomponent 0.0))

(event `self.StopShakingSound_BP`)

(event `self.PlayFallSound_BP`
  (bind _audiocomponent (`self.audioComponent`))
  (`AudioComponent.SetSound` _audiocomponent "/Game/SpaceSchoolAdventure/Sounds/Character/FallingPlatformFall.FallingPlatformFall")
  (`AudioComponent.Play` _audiocomponent 0.5))

(event `self.StopFallSound_BP`
  (bind _audiocomponent (`self.audioComponent`))
  (`AudioComponent.Stop` _audiocomponent)
  (`AudioComponent.SetSound` _audiocomponent null))

(fn `UserConstructionScript`)