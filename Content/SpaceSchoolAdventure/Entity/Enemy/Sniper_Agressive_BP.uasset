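; Aggressive sniper enemy Blueprint for Space School Adventure, providing the enemy's sound and visual feedback.
; Events for attack hurt, jump hurt and hitting the player each play their own sound at the actor's location.
; Tick polls the controller's blackboard every frame and shows the Niagara effect only while IsChasingEnemy is true.
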(event `self.PlayAttackHurtSound_BP`
  (`GameplayStatics.PlaySoundAtLocation` "/Game/SpaceSchoolAdventure/Sounds/Character/EnemyAttackHit.EnemyAttackHit" (`self.K2_GetActorLocation`) (struct) 1.0 1.0 0.0 null null null))

(event `self.ReceiveTick`
  (params (DeltaSeconds :type "Float (single-precision)"))
  (`SceneComponent.SetVisibility` (`self.Niagara`) (`BlackboardComponent.GetValueAsBool` (`AIBlueprintHelperLibrary.GetBlackboard` (`self.GetController`)) (`self.IsChasingEnemy`)) false))

(event `self.PlayJumpHurtSound_BP`
  (`GameplayStatics.PlaySoundAtLocation` "/Game/SpaceSchoolAdventure/Sounds/Character/EnemyJumpHit.EnemyJumpHit" (`self.K2_GetActorLocation`) (struct) 1.0 1.0 0.0 null null null))

(event `self.EnemyHitPlayer_BP`
  (`GameplayStatics.PlaySoundAtLocation` "/Game/SpaceSchoolAdventure/Sounds/Character/EnemyHitPlayer.EnemyHitPlayer" (`self.K2_GetActorLocation`) (struct) 1.0 1.0 0.0 null null null))

(fn `UserConstructionScript`)